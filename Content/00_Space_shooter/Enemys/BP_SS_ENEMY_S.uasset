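; BP_SS_ENEMY_S is a space shooter enemy that moves sideways while firing twin shots on a timer.
; On BeginPlay it caches its right vector, which MoveTorreta uses each Tick to move it at Speed without sweeping.
; Tick also accumulates time and, past FireDelay, calls FireTorreta to spawn Ammo at both fire points, rotated to match the enemy.
; IsRight is set at start but never read here, and nothing reverses the movement.
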(event `self.ReceiveBeginPlay`
  (`parent.ReceiveBeginPlay`)
  (set `self.MovementVector` (`self.GetActorRightVector`))
  (set `self.IsRight` true))

(event `self.ReceiveTick`
  (params (DeltaSeconds :type "Float (single-precision)"))
  (`self.MoveTorreta` DeltaSeconds)
  (bind _output_get (set `self.ShotCurrentTime` (+ DeltaSeconds (`self.ShotCurrentTime`))))
  (if (> _output_get (`self.FireDelay`))
    (set `self.ShotCurrentTime` 0.0)
    (`self.FireTorreta`)))

(fn `FireTorreta`
  (bind _returnvalue (`|SpawnActorFromClass` (`self.Ammo`) (`SceneComponent.K2_GetComponentToWorld` (`self.FirePoint2`)) "Undefined" "MultiplyWithRoot" null null))
  (`self.K2_SetActorRotation` _returnvalue (`self.K2_GetActorRotation`) false)
  (bind _returnvalue_2 (`|SpawnActorFromClass` (`self.Ammo`) (`SceneComponent.K2_GetComponentToWorld` (`self.FirePoint1`)) "Undefined" "MultiplyWithRoot" null null))
  (`self.K2_SetActorRotation` _returnvalue_2 (`self.K2_GetActorRotation`) false))

(fn `MoveTorreta`
  (params (DeltaTime :type "Float (double-precision)"))
  (`self.K2_SetActorLocation` (+ (`self.K2_GetActorLocation`) (* (* DeltaTime (`self.Speed`)) (`self.MovementVector`)))))

(fn `UserConstructionScript`
  (`parent.UserConstructionScript`))