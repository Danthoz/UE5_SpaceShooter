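; Enemy projectile for the space shooter that damages the player on contact.
; Tick moves it along its forward vector at Speed, without sweeping.
; Overlapping an actor tagged Player spawns an explosion, calls DamageActor on player 0's BP_SS_CHARACTER rather than the overlapped actor, plays a sound and destroys the projectile after a short delay.
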(event `self.ReceiveActorBeginOverlap`
  (params (OtherActor :type "Actor Object Reference"))
  (if (`KismetArrayLibrary.Array_Contains` (`Actor.Tags` OtherActor) "Player")
    (`GameplayStatics.SpawnEmitterAtLocation` "/Game/StarterContent/Particles/P_Explosion.P_Explosion" (`self.K2_GetActorLocation`))
    (bind _asbp_ss_character (cast `/Game/00_Space_shooter/Players/BP_SS_CHARACTER` (`GameplayStatics.GetPlayerCharacter` 0)))
    (`/Game/00_Space_shooter/Players/BP_SS_CHARACTER.DamageActor` _asbp_ss_character)
    (`GameplayStatics.PlaySound2D` "/Game/StarterContent/Audio/Explosion01.Explosion01" 1.0 1.0 0.0 null null)
    (`KismetSystemLibrary.Delay` 0.1)
    (`self.K2_DestroyActor`)))

(event `self.ReceiveTick`
  (params (DeltaSeconds :type "Float (single-precision)"))
  (`self.K2_SetActorLocation` (+ (* (* DeltaSeconds (`self.Speed`)) (`self.GetActorForwardVector`)) (`self.K2_GetActorLocation`))))

(fn `UserConstructionScript`)