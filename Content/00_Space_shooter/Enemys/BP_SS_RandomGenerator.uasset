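; BP_SS_RandomGenerator is the enemy spawner for the space shooter, creating enemies on a looping timer while the game mode's level is below 7.
; A level change delays 3 seconds before updating the tracked level, pausing spawns.
; A level-bounded random roll selects one of three enemy classes and a matching range of tagged spawn points.
; Enemy-destroyed events decrement SpawnTime, but the timer is never reset with it.
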(event `self.ReceiveBeginPlay`
  (`KismetSystemLibrary.K2_SetTimerDelegate` (delegate `Spawn`) (`self.SpawnTime`) true)
  (bind _asbp_ss_game_mode (cast `/Game/00_Space_shooter/BP_SS_GameMode` (`GameplayStatics.GetGameMode`)))
  (set `self.m_Game Mode` _asbp_ss_game_mode))

(event `Spawn`
  (bind _level (`/Game/00_Space_shooter/BP_SS_GameMode.Level` (`self.m_Game Mode`)))
  (if (== _level (`self.CurrentLevel`))
    (if (< _level 7)
      ;[1 1 1] Spawn Enemy
      (bind _enemyspawned (`self.SpawnEnemy`))
      (bind _asbp_ss_enemy (cast `/Game/00_Space_shooter/Enemys/BP_SS_ENEMY` _enemyspawned))
      (add `/Game/00_Space_shooter/Enemys/BP_SS_ENEMY.OnEnemyDestroy` _asbp_ss_enemy (delegate `EnemyDestroyed`)))
    (else
      ;[1 1 1] Pausa entre niveles
      (`KismetSystemLibrary.Delay` 3.0)
      (set `self.CurrentLevel` _level))))

(event `EnemyDestroyed`
  ;[1 1 1] Spawn Enemy
  (set `self.SpawnTime` (- (`self.SpawnTime`) 1.0)))

(fn `GetClassToSpawn`
  (params (Type :type Integer))
  (returns (EnemyType :type "/Game/00_Space_shooter/Enemys/BP_SS_ENEMY Class Reference"))
  (bind _returnvalue (`KismetMathLibrary.Clamp` Type 0 (- (`self.MaxNumEnemies`) 1)))
  (if (> _returnvalue 0)
    (set `self.NumPointSpawn` (`KismetMathLibrary.RandomIntegerInRange` 5 9))
    (else
      (set `self.NumPointSpawn` (`KismetMathLibrary.RandomIntegerInRange` 0 4))))
  (return (select `int` _returnvalue :`0` "/Game/00_Space_shooter/Enemys/BP_SS_ENEMY.BP_SS_ENEMY_C" :`1` "/Game/00_Space_shooter/Enemys/BP_SS_ENEMY_H.BP_SS_ENEMY_H_C" :`2` "/Game/00_Space_shooter/Enemys/BP_SS_ENEMY_S.BP_SS_ENEMY_S_C" :!type "/Game/00_Space_shooter/Enemys/BP_SS_ENEMY Class Reference")))

(fn `SpawnEnemy`
  (returns (EnemySpawned :type "/Game/00_Space_shooter/Enemys/BP_SS_ENEMY Object Reference"))
  (bind _enemytype (`self.GetClassToSpawn` (`KismetMathLibrary.RandomInteger` (`/Game/00_Space_shooter/BP_SS_GameMode.Level` (`self.m_Game Mode`)))))
  (bind _returnvalue (`|SpawnActorFromClass` _enemytype (`SceneComponent.K2_GetComponentToWorld` (`|GetArrayItem` (`self.GetComponentsByTag` "/Script/Engine.SceneComponent" "SpawnPoint") (`self.NumPointSpawn`))) "AdjustIfPossibleButAlwaysSpawn" "MultiplyWithRoot" null null))
  (bind _asbp_ss_enemy (cast `/Game/00_Space_shooter/Enemys/BP_SS_ENEMY` _returnvalue))
  (return _asbp_ss_enemy))

(fn `UserConstructionScript`)