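; Boss enemy for the space shooter that reports its spawn, damage and death to BP_SS_GameMode.
; It flies in with collision briefly disabled, then Tick drives a sine-based weaving movement and timed volleys from four fire points.
; Overlaps with "Player"-tagged actors remove lives; an overlap at zero lives fires the OnEnemyDestroy dispatcher, whose bound handler destroys the boss after a short delay.
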(event `self.ReceiveBeginPlay`
  (set `self.BossLifes` 3)
  ;[1 1 1] Avisa al HUD que el boss Spawneo para mostrar vidas
  (bind _asbp_ss_game_mode (cast `/Game/00_Space_shooter/BP_SS_GameMode` (`GameplayStatics.GetGameMode`)))
  (`/Game/00_Space_shooter/BP_SS_GameMode.BossSpawnGM` _asbp_ss_game_mode)
  ;[1 1 1] Permite la entrada del boss sin morir
  (`self.SetActorEnableCollision` false)
  (set `self.SpawnTime` (`KismetSystemLibrary.GetGameTimeInSeconds`))
  (set `self.MovementVector` (`self.GetActorForwardVector`))
  ;[1 1 1] Reactiva hitbox del boss
  (`KismetSystemLibrary.Delay` 5.0)
  (`self.SetActorEnableCollision` true)
  (add `self.OnEnemyDestroy` (delegate `DestroyBoss`)))

(event `DestroyBoss`
  (`KismetSystemLibrary.Delay` 0.1)
  (`self.K2_DestroyActor`))

(event `self.ReceiveActorBeginOverlap`
  (params (OtherActor :type "Actor Object Reference"))
  (bind _bosslifes (`self.BossLifes`))
  (if (`KismetArrayLibrary.Array_Contains` (`Actor.Tags` OtherActor) "Player")
    (if (< _bosslifes 1)
      (`self.OnEnemyDestroy`)
      (bind _asbp_ss_game_mode (cast `/Game/00_Space_shooter/BP_SS_GameMode` (`GameplayStatics.GetGameMode`)))
      (`/Game/00_Space_shooter/BP_SS_GameMode.BossDead` _asbp_ss_game_mode)
      (else
        (set `self.BossLifes` (- _bosslifes 1))
        (bind _asbp_ss_game_mode_2 (cast `/Game/00_Space_shooter/BP_SS_GameMode` (`GameplayStatics.GetGameMode`)))
        (`/Game/00_Space_shooter/BP_SS_GameMode.BossDMDGM` _asbp_ss_game_mode_2)))))

(event `self.ReceiveTick`
  (params (DeltaSeconds :type "Float (single-precision)"))
  (`self.Move` DeltaSeconds)
  (bind _output_get (set `self.ShotCurrentTime` (+ DeltaSeconds (`self.ShotCurrentTime`))))
  (if (> _output_get (`self.FireDelay`))
    (set `self.ShotCurrentTime` 0.0)
    (`self.Fire`)))

(fn `Fire`
  (if (not (< (- (`KismetSystemLibrary.GetGameTimeInSeconds`) (`self.SpawnTime`)) 3.0))
    (bind _returnvalue (`|SpawnActorFromClass` (`self.Ammo`) (`SceneComponent.K2_GetComponentToWorld` (`self.FirePoint1`)) "Undefined" "MultiplyWithRoot" null null))
    (`self.K2_SetActorRotation` _returnvalue (`self.K2_GetActorRotation`) false)
    (bind _returnvalue_2 (`|SpawnActorFromClass` (`self.Ammo`) (`SceneComponent.K2_GetComponentToWorld` (`self.FirePoint2`)) "Undefined" "MultiplyWithRoot" null null))
    (`self.K2_SetActorRotation` _returnvalue_2 (`self.K2_GetActorRotation`) false)
    (bind _returnvalue_3 (`|SpawnActorFromClass` (`self.Ammo`) (`SceneComponent.K2_GetComponentToWorld` (`self.FirePoint3`)) "Undefined" "MultiplyWithRoot" null null))
    (`self.K2_SetActorRotation` _returnvalue_3 (`self.K2_GetActorRotation`) false)
    (bind _returnvalue_4 (`|SpawnActorFromClass` (`self.Ammo`) (`SceneComponent.K2_GetComponentToWorld` (`self.FirePoint4`)) "Undefined" "MultiplyWithRoot" null null))
    (`self.K2_SetActorRotation` _returnvalue_4 (`self.K2_GetActorRotation`) false)))

(fn `Move`
  (params (`Delta Time` :type "Float (double-precision)"))
  (if (< (- (`KismetSystemLibrary.GetGameTimeInSeconds`) (`self.SpawnTime`)) 3.0)
    ;[1 1 1] Movimiento de entrada del boss
    (`self.K2_SetActorLocation` (+ (`self.K2_GetActorLocation`) (* (* `Delta Time` (`self.Speed`)) (`self.GetActorForwardVector`))))
    (elif (not (< (- (`KismetSystemLibrary.GetGameTimeInSeconds`) (`self.SpawnTime`)) 2.5))
      ;[1 1 1] Patron de movimiento del Boss
      (`self.K2_SetActorLocation` (+ (+ (`self.K2_GetActorLocation`) (* (* `Delta Time` (* (`self.Speed`) 2.0)) (* (* (`KismetMathLibrary.Sin` (`KismetSystemLibrary.GetGameTimeInSeconds`)) 1.0) (`self.GetActorRightVector`)))) (* (* (`KismetMathLibrary.Sin` (`KismetSystemLibrary.GetGameTimeInSeconds`)) 1.0) (`self.GetActorForwardVector`)))))))

(fn `UserConstructionScript`)