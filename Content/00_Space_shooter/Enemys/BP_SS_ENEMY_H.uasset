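; BP_SS_ENEMY_H is a space shooter enemy variant whose movement direction alternates between its right and left.
; It sets MovementVector to the actor's right vector at BeginPlay, then flips it, tracked by IsRight, whenever it overlaps an actor tagged "Lateral".
; It calls the parent events and only sets the direction; no code here applies the movement, and its Tick node is disabled.
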(event `self.ReceiveBeginPlay`
  (`parent.ReceiveBeginPlay`)
  (set `self.MovementVector` (`self.GetActorRightVector`))
  (set `self.IsRight` true))

(event `self.ReceiveActorBeginOverlap`
  (params (OtherActor :type "Actor Object Reference"))
  (bind _returnvalue (`self.GetActorRightVector`))
  (`parent.ReceiveActorBeginOverlap` OtherActor)
  (if (`KismetArrayLibrary.Array_Contains` (`Actor.Tags` OtherActor) "Lateral")
    (if (`self.IsRight`)
      (set `self.IsRight` false)
      (set `self.MovementVector` (* -1 _returnvalue))
      (else
        (set `self.IsRight` true)
        (set `self.MovementVector` _returnvalue)))))

(fn `UserConstructionScript`
  (`parent.UserConstructionScript`))