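; Game mode for the space shooter that tracks score, level and enemy kills and relays key game events to the HUD.
; Score rises every tick by a fixed increment, and every third destroyed enemy raises the level.
; Player death and boss spawn, damage and death events each cast the first player's HUD to BP_SS_HUD and call its matching function.
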(event `self.ReceiveTick`
  (params (DeltaSeconds :type "Float (single-precision)"))
  (set `self.Score` (+ (`self.Score`) (`self.IncrementPerTick`))))

(event `PlayerDead`
  (bind _asbp_ss_hud (cast `/Game/00_Space_shooter/UI/BP_SS_HUD` (`PlayerController.GetHUD` (`GameplayStatics.GetPlayerController` 0))))
  (`/Game/00_Space_shooter/UI/BP_SS_HUD.PlayerKilled` _asbp_ss_hud))

(event `Enemy Destroyed`
  (bind _output_get (set `self.EnemiesDestroyed` (+ (`self.EnemiesDestroyed`) 1)))
  (if (== (mod _output_get 3) 0)
    (set `self.Level` (+ (`self.Level`) 1))))

(event `BossDead`
  (bind _asbp_ss_hud (cast `/Game/00_Space_shooter/UI/BP_SS_HUD` (`PlayerController.GetHUD` (`GameplayStatics.GetPlayerController` 0))))
  (`/Game/00_Space_shooter/UI/BP_SS_HUD.BossKilled` _asbp_ss_hud))

(event `BossDMDGM`
  (bind _asbp_ss_hud (cast `/Game/00_Space_shooter/UI/BP_SS_HUD` (`PlayerController.GetHUD` (`GameplayStatics.GetPlayerController` 0))))
  (`/Game/00_Space_shooter/UI/BP_SS_HUD.BossDMG` _asbp_ss_hud))

(event `BossSpawnGM`
  (bind _asbp_ss_hud (cast `/Game/00_Space_shooter/UI/BP_SS_HUD` (`PlayerController.GetHUD` (`GameplayStatics.GetPlayerController` 0))))
  (`/Game/00_Space_shooter/UI/BP_SS_HUD.BossSpawnHUD` _asbp_ss_hud))

(fn `UserConstructionScript`)